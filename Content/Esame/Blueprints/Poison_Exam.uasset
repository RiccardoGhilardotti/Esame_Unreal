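; Poison pickup for the exam game that changes the player's score and can kill them.
; On overlap with the third-person character, it reads its type and points from the Poison row of DT_Exam and passes the points to the character's ExamUi.
; It then hides itself and disables its collision.
; If the total drops below zero, it flags the character to die, disables input, and after a delay deletes it and opens Lvl_ThirdPerson.
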(event Collision|EventActorBeginOverlap
  (params (OtherActor :type Actor%20Object%20Reference))
  (bind _asbp_third_person_character (Utilities|Casting|CastToBP_ThirdPersonCharacter OtherActor))
  (bind _returnvalue (Utilities|GetDataTableRow "/Game/Esame/Blueprints/Datatable/DT_Exam.DT_Exam" "Poison")
    (:then
      (Variables|Default|SetItemType (.type _returnvalue))
      (bind _output_get (Variables|Default|SetCoins (.points _returnvalue)))
      (Default|PointModifier (Variables|/Game/ThirdPerson/Blueprints/BP_ThirdPersonCharacter.BP_ThirdPersonCharacter_C|GetExam_Ui _asbp_third_person_character) _output_get)
      (Rendering|SetVisibility (Variables|Default|GetPoison) false false)
      (Collision|SetCollisionEnabled (Variables|Default|GetSphere) "NoCollision")
      (if (< (Variables|/Game/Esame/Ui/WBP_UI_Exam.WBP_UI_Exam_C|GetTotal_Points (Variables|/Game/ThirdPerson/Blueprints/BP_ThirdPersonCharacter.BP_ThirdPersonCharacter_C|GetExam_Ui _asbp_third_person_character)) 0)
        (Variables|/Game/ThirdPerson/Blueprints/BP_ThirdPersonCharacter.BP_ThirdPersonCharacter_C|SetCanDie _asbp_third_person_character true)
        (Input|DisableInput _asbp_third_person_character (Game|GetPlayerController 0))
        (Utilities|FlowControl|Delay 2.5)
        (Default|Delete _asbp_third_person_character)
        (Game|OpenLevel(byName) "Lvl_ThirdPerson")))))

(fn ConstructionScript)