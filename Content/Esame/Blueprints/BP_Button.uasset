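; BP_Button is an interactable button for a puzzle in which two presses must overlap to stay latched.
; On interaction it raises ButtonCounter in BP_ThirdPersonGameMode, switches to its lit material and calls DoorOpen on its Pressed reference.
; After a six-second delay it reverts the count, pressed flag and material unless the counter equals two.
; Its CanInteract function always returns false.
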(event EventOnInteraction
  (params (OtherActors :type BP%20Third%20Person%20Character%20Object%20Reference))
  (if (not (Variables|Default|GetIsPressed))
    (bind _asbp_third_person_game_mode (Utilities|Casting|CastToBP_ThirdPersonGameMode (Game|GetGameMode)))
    (Variables|/Game/ThirdPerson/Blueprints/BP_ThirdPersonGameMode.BP_ThirdPersonGameMode_C|SetButtonCounter _asbp_third_person_game_mode (+ (Variables|/Game/ThirdPerson/Blueprints/BP_ThirdPersonGameMode.BP_ThirdPersonGameMode_C|GetButtonCounter _asbp_third_person_game_mode) 1))
    (Variables|Default|SetIsPressed true)
    (Rendering|Material|SetMaterial (Variables|Default|GetCylinder) 0 "/Game/Esame/Material/Bottone_On.Bottone_On")
    (Default|DoorOpen (Variables|Default|GetPressed))
    (Utilities|FlowControl|Delay 6.0)
    (if (not (== (Variables|/Game/ThirdPerson/Blueprints/BP_ThirdPersonGameMode.BP_ThirdPersonGameMode_C|GetButtonCounter _asbp_third_person_game_mode) 2))
      (Variables|/Game/ThirdPerson/Blueprints/BP_ThirdPersonGameMode.BP_ThirdPersonGameMode_C|SetButtonCounter _asbp_third_person_game_mode (- (Variables|/Game/ThirdPerson/Blueprints/BP_ThirdPersonGameMode.BP_ThirdPersonGameMode_C|GetButtonCounter _asbp_third_person_game_mode) 1))
      (Variables|Default|SetIsPressed false)
      (Rendering|Material|SetMaterial (Variables|Default|GetCylinder) 0 "/Game/Esame/Material/Bottone_Off.Bottone_Off"))))

(fn ConstructionScript)

(fn CanInteract
  (return false))